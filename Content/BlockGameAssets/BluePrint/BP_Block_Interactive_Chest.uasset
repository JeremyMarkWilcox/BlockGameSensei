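; Interactive chest block that opens and closes its lid when interacted with.
; Each interaction alternates through a FlipFlop between playing and reversing the OpenClosedChest timeline.
; The timeline's OpenAmount drives the pitch of the Pivot component.
; A material copy from Block to Top exists but is never executed.
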(event `self.ReceiveBeginPlay`
  (`parent.ReceiveBeginPlay`))

(event `self.Interact`
  (`/Engine/EditorBlueprintResources/StandardMacros.FlipFlop`
    (:`A`
      (bind (_direction _openamount) (`Timeline|OpenClosedChest` :!label _label)
        (:`Update`
          (`SceneComponent.K2_SetRelativeRotation` (`self.Pivot`) (`KismetMathLibrary.MakeRotator` 0.0 _openamount) false false))))
    (:`B`
      (goto _label :!via `Reverse`))))

(fn `UserConstructionScript`
  (`parent.UserConstructionScript`))