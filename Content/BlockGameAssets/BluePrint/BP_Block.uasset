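; BP_Block is a block actor that breaks over time, showing progress through its material before destroying itself.
; On BeginPlay it creates a dynamic material instance for the Block component and sets the timeline's play rate from DestroyRate.
; StartDestroy plays DestroyTimeline from the start, driving the "Destroy Amount" parameter and destroying the actor on completion.
; StopDestroy cancels this by zeroing the parameter and stopping the timeline.
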(event `self.ReceiveBeginPlay`
  (bind _block (`self.Block`))
  (bind _returnvalue (`PrimitiveComponent.CreateDynamicMaterialInstance` _block 0 (`PrimitiveComponent.GetMaterial` _block 0) "None"))
  (set `self.BlockMat` _returnvalue)
  (`TimelineComponent.SetPlayRate` (`self.DestroyTimeline`) (`self.Destroy Rate`)))

(event `Start Destroy`
  (bind (_direction _destroy_amount) (`Timeline|DestroyTimeline` :!via `PlayFromStart` :!label _label)
    (:`Update`
      (`MaterialInstanceDynamic.SetScalarParameterValue` (`self.BlockMat`) "Destroy Amount" _destroy_amount))
    (:`Finished`
      (`self.K2_DestroyActor`))))

(event `Stop Destroy`
  (`MaterialInstanceDynamic.SetScalarParameterValue` (`self.BlockMat`) "Destroy Amount" 0.0)
  (goto _label :!via `Stop`))

(fn `UserConstructionScript`)